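; BP_EnemyPaddle is an enemy paddle that chases the ball along the world X axis.
; Each Tick, while BallRef is valid, it compares the ball's X position to its own and adds full movement input toward it.
; There is no dead zone, so input is always positive or negative, never zero.
; BallRef is not assigned anywhere in these graphs.
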(event `self.ReceiveTick`
  (params (DeltaSeconds :type "Float (single-precision)"))
  (bind _returnvalue_x (`KismetMathLibrary.BreakVector` (`self.K2_GetActorLocation`)))
  (bind _ballref (`self.BallRef`))
  (bind _returnvalue_x_2 (`KismetMathLibrary.BreakVector` (`self.K2_GetActorLocation` _ballref)))
  (`parent.ReceiveTick` DeltaSeconds)
  (`/Engine/EditorBlueprintResources/StandardMacros.IsValid` _ballref
    (:`Is Valid`
      (`self.AddMovementInput` (`KismetMathLibrary.MakeVector` (`KismetMathLibrary.SelectFloat` 1.0 -1.0 (> (- _returnvalue_x_2 _returnvalue_x) 0.0)))))))

(fn `UserConstructionScript`
  (`parent.UserConstructionScript`))