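; Player paddle pawn for a ball-and-paddle game, also handling game UI setup and game over.
; BeginPlay adds the Enhanced Input context and game HUD, and IA_Move feeds the movement component.
; Ball hits briefly switch off the ball component's collision, apparently to debounce repeat contacts.
; GameOver disables input, destroys the ball, shows the game-over widget and switches to UI-only input with a cursor.
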(event `self.ReceiveBeginPlay`
  (bind _returnvalue (`GameplayStatics.GetPlayerController` 0))
  (bind _asplayer_controller (cast `PlayerController` (`self.GetController`)))
  (bind _returnvalue_2 (pcsubsystem `EnhancedInputLocalPlayerSubsystem` _asplayer_controller))
  (`/Engine/EditorBlueprintResources/StandardMacros.IsValid` _returnvalue_2
    (:`Is Valid`
      (`EnhancedInputSubsystemInterface.AddMappingContext` _returnvalue_2 "/Game/Input/IMC_PlayerActions.IMC_PlayerActions" 0 (struct))
      (bind _returnvalue_3 (`|GenericCreateObject` "/Game/W_GameUI.W_GameUI_C"))
      (`UserWidget.AddToViewport` _returnvalue_3 0)
      (`WidgetBlueprintLibrary.SetInputMode_GameOnly` _returnvalue)
      (set `PlayerController.bShowMouseCursor` false _returnvalue))))

(event `EnhancedInput|/Game/Input/IA_Move`
  (params (ActionValue :type "Float (double-precision)") (ElapsedSeconds :type "Float (double-precision)") (TriggeredSeconds :type "Float (double-precision)") (InputAction :type "InputAction Object Reference" :default "/Game/Input/IA_Move.IA_Move"))
  (:`Triggered`
    (`PawnMovementComponent.AddInputVector` (`self.MovementComp`) (`KismetMathLibrary.MakeVector` ActionValue) false)))

(event `self.Collider.OnComponentHit`
  (params (HitComponent :type "PrimitiveComponent Object Reference") (OtherActor :type "Actor Object Reference") (OtherComp :type "PrimitiveComponent Object Reference") (NormalImpulse :type "Vector Structure") (Hit :type "HitResult Structure (by ref)"))
  (cast `/Game/BP_Ball` OtherActor)
  (`PrimitiveComponent.SetCollisionEnabled` OtherComp "NoCollision")
  (`KismetSystemLibrary.Delay` 0.2)
  (`PrimitiveComponent.SetCollisionEnabled` OtherComp "QueryAndPhysics"))

(event `self.GameOver`
  (bind _returnvalue (`GameplayStatics.GetPlayerController` 0))
  (`self.DisableInput` null)
  (bind _returnvalue_2 (`GameplayStatics.GetActorOfClass` "/Game/BP_Ball.BP_Ball_C"))
  (`self.K2_DestroyActor` _returnvalue_2)
  (bind _returnvalue_3 (`|CreateWidget` "/Game/W_GameOver.W_GameOver_C"))
  (`UserWidget.AddToViewport` _returnvalue_3 0)
  (`WidgetBlueprintLibrary.SetInputMode_UIOnlyEx` _returnvalue null)
  (set `PlayerController.bShowMouseCursor` true _returnvalue))

(fn `UserConstructionScript`)